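; BP_Outline is a Blueprint that shows a static mesh and can add or remove a colored outline around it on demand.
; BeginPlay assigns the configured mesh to the main component.
; CreateOutline spawns a second, unattached copy at the same world transform, with a dynamic outline material driven by color and scale variables.
; DeleteOutline destroys that copy, and a flag prevents duplicate outlines.
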(event `self.ReceiveBeginPlay`
  (`StaticMeshComponent.SetStaticMesh` (`self.myStaticMesh`) (`self.myNewMesh`)))

(event `Create Outline`
  (if (not (`self.HasOutline`))
    (bind _returnvalue (`AddComponent|NODE_AddStaticMeshComponent-0` :`bManualAttachment` true :`RelativeTransform` (`SceneComponent.K2_GetComponentToWorld` (`self.myStaticMesh`))))
    (bind _output_get (set `self.myMeshComponent` _returnvalue))
    (`StaticMeshComponent.SetStaticMesh` _output_get (`self.myNewMesh`))
    (bind _returnvalue_2 (`PrimitiveComponent.CreateDynamicMaterialInstance` _output_get 0 "/Game/DeckAndCards/Meshes/materials/mat_outline.mat_outline" "None"))
    (`MaterialInstanceDynamic.SetVectorParameterValue` _returnvalue_2 "Color" (`self.myColor`))
    (`MaterialInstanceDynamic.SetScalarParameterValue` _returnvalue_2 "Scale" (`self.myScale`))
    (set `self.HasOutline` true)))

(event `Delete Outline`
  (bind _mymeshcomponent (`self.myMeshComponent`))
  (`/Engine/EditorBlueprintResources/StandardMacros.IsValid` _mymeshcomponent
    (:`Is Valid`
      (`ActorComponent.K2_DestroyComponent` _mymeshcomponent)
      (set `self.HasOutline` false))))

(fn `UserConstructionScript`)