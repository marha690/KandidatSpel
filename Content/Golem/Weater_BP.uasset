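; Weather controller that switches between firestorm, rain, leafstorm, thunderstorm and clear states, notifying two golems to update their crystals.
; ChangeWeatherEffect resets sky, light, particles and audio, then triggers the chosen effect.
; Each storm uses a timeline to blend sky material parameters and activates its audio.
; Rain and leaves add delayed particles, firestorm spawns random meteor projectiles on a timer, and storm light tints are unconnected.
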(event `Spawn meteor`
  ;[1 1 1] Fire Effect
  (if (`self.SpawnMeteors?`)
    (`|SpawnActorFromClass` "/Game/WeatherEffects/Fire/BP_Projectile.BP_Projectile_C" (`KismetMathLibrary.Conv_VectorToTransform` (`KismetMathLibrary.MakeVector` (`KismetMathLibrary.Conv_IntToDouble` (`KismetMathLibrary.RandomIntegerInRange` -3000 3000)) (`KismetMathLibrary.Conv_IntToDouble` (`KismetMathLibrary.RandomIntegerInRange` -3000 3000)) (`KismetMathLibrary.Conv_IntToDouble` (`KismetMathLibrary.RandomIntegerInRange` 2500 3500)))) "Undefined" "OverrideRootScale" null null)))

(event `TriggerFireEffect`
  (bind _sky_material (`/Engine/EngineSky/BP_Sky_Sphere.Sky material` (`self.SkyRef`)))
  ;[1 1 1] Fire Effect
  (`KismetSystemLibrary.PrintString` "Fire effect starts")
  (set `self.SpawnMeteors?` true)
  (if (`KismetSystemLibrary.IsValid` (`self.SkyRef`))
    (`|ExecutionSequence`
      (:`then_0`
        (bind (_direction _newtrack_0) (`Timeline|Timeline_0`)
          (:`Update`
            (`MaterialInstanceDynamic.SetVectorParameterValue` _sky_material "Zenith color" (`KismetMathLibrary.LinearColorLerp` (struct :`R` 0.034046 :`G` 0.109247 :`B` 0.295 :`A` 1.0) (struct :`R` 0.052083 :`G` 0.052083 :`B` 0.052083 :`A` 1.0) _newtrack_0))
            (`MaterialInstanceDynamic.SetVectorParameterValue` _sky_material "Horizon color" (`KismetMathLibrary.LinearColorLerp` (struct :`R` 1.979559 :`G` 2.586644 :`B` 3.0 :`A` 1.0) (struct :`R` 0.057292 :`G` 0.057292 :`B` 0.057292 :`A` 1.0) _newtrack_0))
            (`MaterialInstanceDynamic.SetVectorParameterValue` _sky_material "Cloud color" (`KismetMathLibrary.LinearColorLerp` (struct :`R` 0.855778 :`G` 0.91902 :`B` 1.0 :`A` 1.0) (struct :`R` 0.96875 :`B` 0.010883 :`A` 1.0) _newtrack_0))
            (`MaterialInstanceDynamic.SetScalarParameterValue` _sky_material "Cloud Opacity" (`KismetMathLibrary.Lerp` 1.2 5.0 _newtrack_0)))))
      (:`then_1`
        (`KismetSystemLibrary.K2_SetTimerDelegate` (delegate `Spawn meteor`) 0.25 (`self.SpawnMeteors?`)))
      (:`then_2`
        (`KismetSystemLibrary.Delay` 0.0)
        (`ActorComponent.Activate` (`self.FireAudio`) false)))))

(event `TriggerRainEffect`
  (bind _sky_material (`/Engine/EngineSky/BP_Sky_Sphere.Sky material` (`self.SkyRef`)))
  ;[1 1 1] Rain Effect
  (`KismetSystemLibrary.PrintString` "Rain effect starts")
  (if (`KismetSystemLibrary.IsValid` (`self.SkyRef`))
    (`|ExecutionSequence`
      (:`then_0`
        (bind (_direction _newtrack_0) (`Timeline|Timeline_1`)
          (:`Update`
            (`MaterialInstanceDynamic.SetVectorParameterValue` _sky_material "Zenith color" (`KismetMathLibrary.LinearColorLerp` (struct :`R` 0.034046 :`G` 0.109247 :`B` 0.295 :`A` 1.0) (struct :`R` 0.052083 :`G` 0.052083 :`B` 0.052083 :`A` 1.0) _newtrack_0))
            (`MaterialInstanceDynamic.SetVectorParameterValue` _sky_material "Horizon color" (`KismetMathLibrary.LinearColorLerp` (struct :`R` 1.979559 :`G` 2.586644 :`B` 3.0 :`A` 1.0) (struct :`R` 0.057292 :`G` 0.057292 :`B` 0.057292 :`A` 1.0) _newtrack_0))
            (`MaterialInstanceDynamic.SetVectorParameterValue` _sky_material "Cloud color" (`KismetMathLibrary.LinearColorLerp` (struct :`R` 0.855778 :`G` 0.91902 :`B` 1.0 :`A` 1.0) (struct :`R` 0.017687 :`G` 0.089291 :`B` 0.869792 :`A` 1.0) _newtrack_0))
            (`MaterialInstanceDynamic.SetScalarParameterValue` _sky_material "Cloud Opacity" (`KismetMathLibrary.Lerp` 1.2 5.0 _newtrack_0)))))
      (:`then_1`
        (`KismetSystemLibrary.Delay` 2.0)
        (`ActorComponent.Activate` (`Emitter.ParticleSystemComponent` (`self.RainRef2`)) false)
        (`ActorComponent.Activate` (`Emitter.ParticleSystemComponent` (`self.RainRef1`)) false))
      (:`then_2`
        (`KismetSystemLibrary.Delay` 0.0)
        (`ActorComponent.Activate` (`self.RainAudio`) false)))))

(event `TriggerLeafEffect`
  (bind _sky_material (`/Engine/EngineSky/BP_Sky_Sphere.Sky material` (`self.SkyRef`)))
  ;[1 1 1] Leafstorm Effect
  (if (`KismetSystemLibrary.IsValid` (`self.SkyRef`))
    (`|ExecutionSequence`
      (:`then_0`
        (bind (_direction _newtrack_0) (`Timeline|Timeline_2`)
          (:`Update`
            (`MaterialInstanceDynamic.SetVectorParameterValue` _sky_material "Zenith color" (`KismetMathLibrary.LinearColorLerp` (struct :`R` 0.034046 :`G` 0.109247 :`B` 0.295 :`A` 1.0) (struct :`R` 0.052083 :`G` 0.052083 :`B` 0.052083 :`A` 1.0) _newtrack_0))
            (`MaterialInstanceDynamic.SetVectorParameterValue` _sky_material "Horizon color" (`KismetMathLibrary.LinearColorLerp` (struct :`R` 1.979559 :`G` 2.586644 :`B` 3.0 :`A` 1.0) (struct :`R` 0.057292 :`G` 0.057292 :`B` 0.057292 :`A` 1.0) _newtrack_0))
            (`MaterialInstanceDynamic.SetVectorParameterValue` _sky_material "Cloud color" (`KismetMathLibrary.LinearColorLerp` (struct :`R` 0.855778 :`G` 0.91902 :`B` 1.0 :`A` 1.0) (struct :`R` 0.013664 :`G` 0.270833 :`A` 1.0) _newtrack_0))
            (`MaterialInstanceDynamic.SetScalarParameterValue` _sky_material "Cloud Opacity" (`KismetMathLibrary.Lerp` 1.2 5.0 _newtrack_0)))))
      (:`then_1`
        (`KismetSystemLibrary.Delay` 2.0)
        (`ActorComponent.Activate` (`Emitter.ParticleSystemComponent` (`self.LeafRef2`)) false)
        (`ActorComponent.Activate` (`Emitter.ParticleSystemComponent` (`self.LeafRef1`)) false))
      (:`then_2`
        (`KismetSystemLibrary.Delay` 0.0)
        (`ActorComponent.Activate` (`self.LeafAudio`) false)))))

(event `TriggerThunderEffect`
  (bind _sky_material (`/Engine/EngineSky/BP_Sky_Sphere.Sky material` (`self.SkyRef`)))
  ;[1 1 1] Thunder Effect
  (if (`KismetSystemLibrary.IsValid` (`self.SkyRef`))
    (`|ExecutionSequence`
      (:`then_0`
        (bind (_direction _newtrack_0) (`Timeline|Timeline_3`)
          (:`Update`
            (`MaterialInstanceDynamic.SetVectorParameterValue` _sky_material "Zenith color" (`KismetMathLibrary.LinearColorLerp` (struct :`R` 0.034046 :`G` 0.109247 :`B` 0.295 :`A` 1.0) (struct :`R` 0.052083 :`G` 0.052083 :`B` 0.052083 :`A` 1.0) _newtrack_0))
            (`MaterialInstanceDynamic.SetVectorParameterValue` _sky_material "Horizon color" (`KismetMathLibrary.LinearColorLerp` (struct :`R` 1.979559 :`G` 2.586644 :`B` 3.0 :`A` 1.0) (struct :`R` 0.057292 :`G` 0.057292 :`B` 0.057292 :`A` 1.0) _newtrack_0))
            (`MaterialInstanceDynamic.SetVectorParameterValue` _sky_material "Cloud color" (`KismetMathLibrary.LinearColorLerp` (struct :`R` 0.855778 :`G` 0.91902 :`B` 1.0 :`A` 1.0) (struct :`R` 0.505208 :`G` 0.486442 :`A` 1.0) _newtrack_0))
            (`MaterialInstanceDynamic.SetScalarParameterValue` _sky_material "Cloud Opacity" (`KismetMathLibrary.Lerp` 1.2 5.0 _newtrack_0)))))
      (:`then_1`
        (`ActorComponent.Activate` (`self.ThunderAudio`) false)))))

(event `TriggerNoWeatherEffect`
  (bind _sky_material (`/Engine/EngineSky/BP_Sky_Sphere.Sky material` (`self.SkyRef`)))
  ;[1 1 1] No weather Effect
  (if (`KismetSystemLibrary.IsValid` (`self.SkyRef`))
    (`|ExecutionSequence`
      (:`then_0`
        (set `self.SpawnMeteors?` false))
      (:`then_1`
        (`MaterialInstanceDynamic.SetVectorParameterValue` _sky_material "Zenith color" (`KismetMathLibrary.SelectColor` (struct :`R` 0.034046 :`G` 0.109247 :`B` 0.295 :`A` 1.0) (struct) true))
        (`MaterialInstanceDynamic.SetVectorParameterValue` _sky_material "Horizon color" (`KismetMathLibrary.SelectColor` (struct :`R` 1.979559 :`G` 2.586644 :`B` 3.0 :`A` 1.0) (struct) true))
        (`MaterialInstanceDynamic.SetVectorParameterValue` _sky_material "Cloud color" (`KismetMathLibrary.SelectColor` (struct :`R` 1.0 :`G` 1.0 :`B` 1.0 :`A` 1.0) (struct) true))
        (`MaterialInstanceDynamic.SetScalarParameterValue` _sky_material "Cloud Opacity" 1.2)
        (`LightComponent.SetLightColor` (`Light.LightComponent` (`self.LightRef`)) (`KismetMathLibrary.SelectColor` (struct :`R` 1.0 :`G` 1.0 :`B` 1.0 :`A` 1.0) (struct) true) true)
        (`ActorComponent.Deactivate` (`Emitter.ParticleSystemComponent` (`self.RainRef1`)))
        (`ActorComponent.Deactivate` (`Emitter.ParticleSystemComponent` (`self.RainRef2`)))
        (`ActorComponent.Deactivate` (`Emitter.ParticleSystemComponent` (`self.LeafRef2`)))
        (`ActorComponent.Deactivate` (`Emitter.ParticleSystemComponent` (`self.LeafRef1`)))
        (`ActorComponent.Deactivate` (`self.LeafAudio`))
        (`ActorComponent.Deactivate` (`self.ThunderAudio`))
        (`ActorComponent.Deactivate` (`self.RainAudio`))
        (`ActorComponent.Deactivate` (`self.FireAudio`))))))

(fn `ChangeWeatherEffect`
  (params (WeatherEffect :type "/Game/Golem/Weather Enum" :default "NewEnumerator3"))
  (bind _output_get (set `self.ActiveWeather` WeatherEffect))
  (`/Game/Golem/Golem_BP.UpdateCrystalsFromWeatherEffect` (`self.Golem1`))
  (`/Game/Golem/Golem_BP.UpdateCrystalsFromWeatherEffect` (`self.Golem2`))
  ;[1 1 1] Removes stuff in scene
  (`self.TriggerNoWeatherEffect`)
  (switch `/Game/Golem/Weather` _output_get
    (:`NewEnumerator3`
      (`self.TriggerFireEffect`))
    (:`NewEnumerator2`
      (`self.TriggerLeafEffect`))
    (:`NewEnumerator0`
      (`self.TriggerThunderEffect`))
    (:`NewEnumerator1`
      (`self.TriggerRainEffect`))
    (:`NewEnumerator4`
      (`self.TriggerNoWeatherEffect`))))

(fn `UserConstructionScript`)