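; Golem combatant that collects four elemental crystals, attacks an enemy golem, blocks and takes damage.
; SetCrystal sets element flags and material slots, and holding all four turns it Spectral.
; Attacks add bonuses for elements the enemy doesn't counter, or a larger Spectral bonus, then clear elements; blocking reduces damage, or heals when Spectral.
; A weather-change event strips the element opposed by the active weather unless Spectral.
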(event `self.ReceiveBeginPlay`
  (add `self.NewEventDispatcher_0` (delegate `WeatherChanged`)))

(event `WeatherChanged`
  ;[1 1 1] Remove elements depending on the weather effect
  (if (not (`self.isSpectral?`))
    (switch `/Game/Golem/Weather` (`/Game/Golem/Weater_BP.ActiveWeather` (`self.Weather_REf`))
      (:`NewEnumerator3`
        (`PrimitiveComponent.SetMaterial` (`self.TempGolem`) 0 "/Game/Geometry/Meshes/CubeMaterial.CubeMaterial") ; Nature
        (set `self.hasNature?` false))
      (:`NewEnumerator2`
        (`PrimitiveComponent.SetMaterial` (`self.TempGolem`) 3 "/Game/Geometry/Meshes/CubeMaterial.CubeMaterial") ; Thunder
        (set `self.hasThunder?` false))
      (:`NewEnumerator0`
        (`PrimitiveComponent.SetMaterial` (`self.TempGolem`) 2 "/Game/Geometry/Meshes/CubeMaterial.CubeMaterial") ; Water
        (set `self.hasWater?` false))
      (:`NewEnumerator1`
        (`PrimitiveComponent.SetMaterial` (`self.TempGolem`) 1 "/Game/Geometry/Meshes/CubeMaterial.CubeMaterial") ; Fire
        (set `self.hasFire?` false)))))

(fn `AttackOtherGolem`
  (params (StrongAttack :type Boolean))
  (locals (Damage :type Integer))
  ;[1 1 1] Physical attack
  (if StrongAttack
    (set `local.Damage` 3)
    (else
      (set `local.Damage` 1)))
  (if (`self.isSpectral?`)
    ;[1 1 1] Spectral Damage
    (set `local.Damage` (+ (`local.Damage`) 6))
    (set `self.isSpectral?` false)
    (else
      ;[1 1 1] Elemental Damage
      ;;[1 1 1] Fire Damage
      (if (`self.hasFire?`)
        (if (not (`/Game/Golem/Golem_BP.hasWater?` (`self.EnemyGolem`)))
          (set `local.Damage` (+ (`local.Damage`) 1))))
      ;;[1 1 1] Nature Damage
      (if (`self.hasNature?`)
        (if (not (`/Game/Golem/Golem_BP.hasFire?` (`self.EnemyGolem`)))
          (set `local.Damage` (+ (`local.Damage`) 1))))
      ;;[1 1 1] Thunder Damage
      (if (`self.hasThunder?`)
        (if (not (`/Game/Golem/Golem_BP.hasNature?` (`self.EnemyGolem`)))
          (set `local.Damage` (+ (`local.Damage`) 1))))
      ;;[1 1 1] Water Damage
      (if (`self.hasWater?`)
        (if (not (`/Game/Golem/Golem_BP.hasThunder?` (`self.EnemyGolem`)))
          (set `local.Damage` (+ (`local.Damage`) 1))))))
  ;[1 1 1] Other golem block reduction from meele
  (if (`/Game/Golem/Golem_BP.isDefending?` (`self.EnemyGolem`))
    (set `local.Damage` (`KismetMathLibrary.Max` (- (`local.Damage`) 2))))
  (`self.TakeDamage` (`self.EnemyGolem`) (`local.Damage`))
  (`self.ResetAllElements`))

(fn `Block`
  (if (`self.isSpectral?`)
    (`self.Heal` 5)
    ;[1 1 1] Heal
    (set `self.isSpectral?` false)
    (`self.ResetAllElements`)
    (elif (not (`self.isDefending?`))
      ;[1 1 1] Block
      (set `self.isDefending?` true)
      (`SceneComponent.SetVisibility` (`self.BlockShield`) true false))))

(fn `Heal`
  (params (HealValue :type Integer))
  (set `self.HP` (`KismetMathLibrary.Min` (+ (`self.HP`) HealValue) (`self.HP_MaxValue`)))
  (return))

(fn `RefreshMaterials`
  (if true
    _))

(fn `ResetAllElements`
  (bind _tempgolem (`self.TempGolem`))
  (bind _tempgolem_2 (`self.TempGolem`))
  (set `self.hasWater?` false)
  (set `self.hasFire?` false)
  (set `self.hasNature?` false)
  (set `self.hasThunder?` false)
  (`PrimitiveComponent.SetMaterial` _tempgolem_2 0 "/Game/Geometry/Meshes/CubeMaterial.CubeMaterial")
  (`PrimitiveComponent.SetMaterial` _tempgolem_2 0 "/Game/Geometry/Meshes/CubeMaterial.CubeMaterial")
  (`PrimitiveComponent.SetMaterial` _tempgolem 0 "/Game/Geometry/Meshes/CubeMaterial.CubeMaterial")
  (`PrimitiveComponent.SetMaterial` _tempgolem 0 "/Game/Geometry/Meshes/CubeMaterial.CubeMaterial"))

(fn `SetCrystal`
  (params (Element :type "/Game/Golem/Crystal Enum" :default "NewEnumerator0"))
  (locals (ElementIn :type "/Game/Golem/Crystal Enum" :default "NewEnumerator0") (Index :type Integer))
  (bind _tempgolem (`self.TempGolem`))
  (bind _output_get (set `local.ElementIn` Element))
  (switch `/Game/Golem/Crystal` _output_get
    (:`NewEnumerator2`
      (if (not (`self.hasFire?`))
        (`PrimitiveComponent.SetMaterial` (`self.TempGolem`) 1 "/Game/Materials/Material_FireStone.Material_FireStone")
        (set `self.hasFire?` true)
        (if (and (`self.hasWater?`) (`self.hasFire?`) (`self.hasNature?`) (`self.hasThunder?`)) :!label _label
          (set `self.isSpectral?` true)
          (`PrimitiveComponent.SetMaterial` _tempgolem 0 "/Game/Materials/Spectral.Spectral")
          (`PrimitiveComponent.SetMaterial` _tempgolem 1 "/Game/Materials/Spectral.Spectral")
          (`PrimitiveComponent.SetMaterial` _tempgolem 2 "/Game/Materials/Spectral.Spectral")
          (`PrimitiveComponent.SetMaterial` _tempgolem 3 "/Game/Materials/Spectral.Spectral"))))
    (:`NewEnumerator1`
      (if (not (`self.hasNature?`))
        (`PrimitiveComponent.SetMaterial` (`self.TempGolem`) 0 "/Game/Materials/Material_NatureStone.Material_NatureStone") ; Nature
        (set `self.hasNature?` true)
        (goto _label)))
    (:`NewEnumerator3`
      (if (not (`self.hasThunder?`))
        (`PrimitiveComponent.SetMaterial` (`self.TempGolem`) 3 "/Game/Materials/Material_ThunderStone.Material_ThunderStone")
        (set `self.hasThunder?` true)
        (goto _label)))
    (:`NewEnumerator0`
      (if (not (`self.hasWater?`))
        (`PrimitiveComponent.SetMaterial` (`self.TempGolem`) 2 "/Game/Materials/Material_WaterStone.Material_WaterStone")
        (set `self.hasWater?` true)
        (goto _label)))))

(fn `TakeDamage`
  (params (Damage :type Integer))
  (set `self.HP` (`KismetMathLibrary.Clamp` (- (`self.HP`) Damage) 0 (`self.HP_MaxValue`)))
  (`KismetSystemLibrary.PrintString` (`KismetStringLibrary.Concat_StrStr` "Golem took " (`KismetStringLibrary.Conv_IntToString` Damage) " damage."))
  (set `self.isDefending?` false)
  (`SceneComponent.SetVisibility` (`self.BlockShield`) false false))

(fn `UserConstructionScript`)